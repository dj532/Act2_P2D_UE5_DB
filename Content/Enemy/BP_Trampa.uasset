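; BP_Trampa is a moving trap that damages the player character on contact.
; On BeginPlay, the MovimientoTrampa timeline drives the actor's location between PuntoTrampA and PuntoTrampB, without sweep.
; When Trampa_Mesh overlaps a BP_ThirdPersonCharacter, it applies DamageTrampa damage and spawns an explosion emitter with no location supplied.
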(event OnComponentBeginOverlap(Trampa_Mesh)
  (params (OverlappedComponent :type Primitive%20Component%20Object%20Reference) (OtherActor :type Actor%20Object%20Reference) (OtherComp :type Primitive%20Component%20Object%20Reference) (OtherBodyIndex :type Integer) (bFromSweep :type Boolean) (SweepResult :type Hit%20Result%20Structure%20%28by%20ref%29))
  (bind _asbp_third_person_character (Utilities|Casting|CastToBP_ThirdPersonCharacter OtherActor))
  (Game|Damage|ApplyDamage _asbp_third_person_character (Variables|Default|GetDamageTrampa) 0 0)
  (Effects|SpawnEmitteratLocation "/Game/StarterContent/Particles/P_Explosion.P_Explosion" "0, 0, 0"))

(event EventBeginPlay
  (bind _sube_baja (Timeline|MovimientoTrampa Play)
    (:Update
      (Transformation|SetActorLocation self (Math|Vector|Lerp(Vector) (Variables|Default|GetPuntoTramp_A) (Variables|Default|GetPuntoTramp_B) _sube_baja) false false))))

(event Collision|EventActorBeginOverlap
  (params (OtherActor :type Actor%20Object%20Reference)))

(event EventTick
  (params (DeltaSeconds :type Float%20%28single-precision%29)))

(fn ConstructionScript)