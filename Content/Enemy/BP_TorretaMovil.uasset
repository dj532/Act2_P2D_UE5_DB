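; BP_TorretaMovil is a moving enemy turret that fires bullets automatically.
; On BeginPlay it runs a timeline in reverse, whose track lerps the actor's location between two points without sweeping.
; Tick spawns BP_Enemy_Bullet at the FirePoint transform, using a CanFire flag and a Delay to limit the fire rate, with no targeting or player check.
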(event EventBeginPlay
  (bind _pistatorreta (Timeline|TimelineTorretaMovil Reverse)
    (:Update
      (Transformation|SetActorLocation self (Math|Vector|Lerp(Vector) (Variables|Default|GetPntoTorretaA) (Variables|Default|GetPntoTorretaB) _pistatorreta) false false))))

(event Collision|EventActorBeginOverlap
  (params (OtherActor :type Actor%20Object%20Reference)))

(event EventTick
  (params (DeltaSeconds :type Float%20%28single-precision%29))
  (if (Variables|Default|GetCanFire)
    (Variables|Default|SetCanFire false)
    (Game|SpawnActorfromClass "/Game/Enemy/BP_Enemy_Bullet.BP_Enemy_Bullet_C" (Transformation|GetWorldTransform (Variables|Default|GetFirePoint)) "Undefined" "MultiplyWithRoot" 0 0)
    (Utilities|FlowControl|Delay (Variables|Default|GetDelayFire))
    (Variables|Default|SetCanFire true)))

(fn ConstructionScript)