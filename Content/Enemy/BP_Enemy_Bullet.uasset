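; BP_Enemy_Bullet is an enemy projectile that damages the third-person player character on contact.
; Tick moves it along its forward vector at Speed, scaled by delta time, without sweeping.
; On overlap with BP_ThirdPersonCharacter it spawns an explosion emitter and applies damage.
; It destroys itself after overlapping any actor, whether or not that actor is the player.
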(event EventBeginPlay)

(event Collision|EventActorBeginOverlap
  (params (OtherActor :type Actor%20Object%20Reference))
  (bind _asbp_third_person_character (Utilities|Casting|CastToBP_ThirdPersonCharacter OtherActor)
    (:then
      (Effects|SpawnEmitteratLocation "/Game/StarterContent/Particles/P_Explosion.P_Explosion" (Transformation|GetActorLocation))
      (Game|Damage|ApplyDamage _asbp_third_person_character 1e+01 0 self))
    (:CastFailed
      _))
  (Actor|DestroyActor))

(event EventTick
  (params (DeltaSeconds :type Float%20%28single-precision%29))
  (Transformation|SetActorLocation (+ (Transformation|GetActorLocation) (* (* (Variables|Default|GetSpeed) DeltaSeconds) (Transformation|GetActorForwardVector))) false false))

(fn ConstructionScript)